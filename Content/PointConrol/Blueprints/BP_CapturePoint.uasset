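; Server-authoritative capture point that a living, player-controlled shooter character claims by staying inside its box for a set duration.
; A looping timer and capsule overlap events drive an Idle, Capturing, Captured state machine held in one struct with player identity and a server-time deadline.
; The first valid occupant becomes sole captor, and leaving or becoming invalid resets progress.
; Captured is final and stops the timer.
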(event `self.ReceiveBeginPlay`
  (`/Engine/EditorBlueprintResources/ActorMacros.Switch Has Authority`
    (:`Authority`
      (bind _returnvalue (`KismetSystemLibrary.K2_SetTimerDelegate` (`|CreateDelegate` :!event `UpdateCapture`) 0.05 true true))
      (set `self.CaptureTimerHandle` _returnvalue)
      (`self.UpdateCapture`))))

(event `self.CaptureBox.OnComponentBeginOverlap`
  (params (OverlappedComponent :type "PrimitiveComponent Object Reference") (OtherActor :type "Actor Object Reference") (OtherComp :type "PrimitiveComponent Object Reference") (OtherBodyIndex :type Integer) (bFromSweep :type Boolean) (SweepResult :type "HitResult Structure (by ref)"))
  (`/Engine/EditorBlueprintResources/ActorMacros.Switch Has Authority`
    (:`Authority`
      (bind _asbp_shooter_character (cast `/Game/ThirdPerson/Blueprints/PointConrolCharacter/BP_ShooterCharacter` OtherActor))
      (if (== (`Character.CapsuleComponent` _asbp_shooter_character) OtherComp)
        (`self.UpdateCapture`)))))

(event `self.CaptureBox.OnComponentEndOverlap`
  (params (OverlappedComponent :type "PrimitiveComponent Object Reference") (OtherActor :type "Actor Object Reference") (OtherComp :type "PrimitiveComponent Object Reference") (OtherBodyIndex :type Integer))
  (`/Engine/EditorBlueprintResources/ActorMacros.Switch Has Authority`
    (:`Authority`
      (if (`|EnumEquality` (`.Phase_3_5C5DC6944A7B4133DE3393BA87121441` (break `/Game/PointConrol/Structures/ST_CaptureState` (`self.CaptureState`))) "NewEnumerator1")
        (if (== OtherActor (`self.ActiveCaptor`))
          (bind _asbp_shooter_character (cast `/Game/ThirdPerson/Blueprints/PointConrolCharacter/BP_ShooterCharacter` OtherActor))
          (if (== (`Character.CapsuleComponent` _asbp_shooter_character) OtherComp)
            (`self.ResetCapture`)))))))

(fn `CanCapture`
  (params (Candidate :type "/Game/ThirdPerson/Blueprints/PointConrolCharacter/BP_ShooterCharacter Object Reference"))
  (returns (`Can Capture` :type Boolean))
  (`/Engine/EditorBlueprintResources/StandardMacros.IsValid` Candidate
    (:`Is Valid`
      (if (`/Game/ThirdPerson/Blueprints/PointConrolCharacter/BP_ShooterCharacter.IsAlive` Candidate)
        (if (`Pawn.IsPlayerControlled` Candidate)
          (`/Engine/EditorBlueprintResources/StandardMacros.IsValid` (`Pawn.PlayerState` Candidate)
            (:`Is Valid`
              (return (`PrimitiveComponent.IsOverlappingComponent` (`self.CaptureBox`) (`Character.CapsuleComponent` Candidate))))
            (:`Is Not Valid`
              _)))))
    (:`Is Not Valid`
      _))
  (return false))

(fn `ResetCapture`
  (set `self.ActiveCaptor` null)
  (set `self.CaptureState` (make `/Game/PointConrol/Structures/ST_CaptureState` "NewEnumerator0")))

(fn `StartCapture`
  (params (Candidate :type "/Game/ThirdPerson/Blueprints/PointConrolCharacter/BP_ShooterCharacter Object Reference"))
  (bind _playerstate (`Pawn.PlayerState` Candidate))
  (set `self.ActiveCaptor` Candidate)
  (set `self.CaptureState` (make `/Game/PointConrol/Structures/ST_CaptureState` "NewEnumerator1" (+ (`GameStateBase.GetServerWorldTimeSeconds` (`GameplayStatics.GetGameState`)) (`self.CaptureDuration`)) (`PlayerState.PlayerId` _playerstate) (`PlayerState.GetPlayerName` _playerstate))))

(fn `UpdateCapture`
  (bind (_phase _endsatservertime _playerid _playername) (break `/Game/PointConrol/Structures/ST_CaptureState` (`self.CaptureState`)))
  (`/Engine/EditorBlueprintResources/ActorMacros.Switch Has Authority`
    (:`Authority`
      (`/Engine/EditorBlueprintResources/StandardMacros.IsValid` (`GameplayStatics.GetGameState`)
        (:`Is Valid`
          (switch `/Game/PointConrol/Blueprints/E_CapturePhase` _phase
            (:`NewEnumerator0`
              (for _array_element (`PrimitiveComponent.GetOverlappingActors` (`self.CaptureBox`) "/Game/ThirdPerson/Blueprints/PointConrolCharacter/BP_ShooterCharacter.BP_ShooterCharacter_C")
                (bind _asbp_shooter_character (cast `/Game/ThirdPerson/Blueprints/PointConrolCharacter/BP_ShooterCharacter` _array_element))
                (bind _can_capture (`self.CanCapture` _asbp_shooter_character))
                (if _can_capture
                  (`self.StartCapture` _asbp_shooter_character)
                  (break))))
            (:`NewEnumerator1`
              (bind _can_capture_2 (`self.CanCapture` (`self.ActiveCaptor`)))
              (if _can_capture_2
                (if (>= (`GameStateBase.GetServerWorldTimeSeconds` (`GameplayStatics.GetGameState`)) _endsatservertime)
                  (set `self.CaptureState` (make `/Game/PointConrol/Structures/ST_CaptureState` "NewEnumerator2" _endsatservertime _playerid _playername))
                  (set `self.ActiveCaptor` null)
                  (`KismetSystemLibrary.K2_ClearAndInvalidateTimerHandle` (`self.CaptureTimerHandle`)))
                (else
                  (`self.ResetCapture`))))))))))

(fn `UserConstructionScript`)